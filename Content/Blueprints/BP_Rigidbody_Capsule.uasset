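; BP_Rigidbody_Capsule is a capsule rigidbody actor whose visible shape and collider are sized from shared Radius and Length values.
; BuildCapsule scales a cylinder child actor and two cap child actors, offsetting the caps to either end along Z.
; It copies the same dimensions to a PositionalCapsuleCollider, and runs both in the construction script and at BeginPlay.
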(event EventBeginPlay
  (CallFunction|BuildCapsule))

(fn ConstructionScript
  (CallFunction|BuildCapsule))

(fn BuildCapsule
  (bind _positionalcapsulecollider (Variables|Default|GetPositionalCapsuleCollider))
  (bind _cap1 (Variables|Default|Getcap1))
  (bind _cap2 (Variables|Default|Getcap2))
  (bind _childactor (Variables|/Script/Engine.ChildActorComponent|GetChildActor _cap1))
  (bind _childactor_2 (Variables|/Script/Engine.ChildActorComponent|GetChildActor _cap2))
  (Transformation|SetActorRelativeScale3D (Variables|/Script/Engine.ChildActorComponent|GetChildActor (Variables|Default|Getcylinder)) (Math|Vector|MakeVector (/ (Variables|Default|GetRadius) 5e+01) (/ (Variables|Default|GetRadius) 5e+01) (/ (Variables|Default|GetLength) 1e+02)))
  (Transformation|SetActorRelativeScale3D _childactor (Math|Vector|MakeVector (/ (Variables|Default|GetRadius) 5e+01) (/ (Variables|Default|GetRadius) 5e+01) (/ (Variables|Default|GetRadius) 5e+01)))
  (Transformation|SetActorRelativeLocation _childactor (Math|Vector|MakeVector 0.0 0.0 (/ (Variables|Default|GetLength) 2.0)))
  (Transformation|SetActorRelativeScale3D _childactor_2 (Math|Vector|MakeVector (/ (Variables|Default|GetRadius) 5e+01) (/ (Variables|Default|GetRadius) 5e+01) (/ (Variables|Default|GetRadius) 5e+01)))
  (Transformation|SetActorRelativeLocation _childactor_2 (Math|Vector|MakeVector 0.0 0.0 (* (/ (Variables|Default|GetLength) 2.0) -1.0)))
  (Variables|/Script/unreal_positional.PositionalCapsuleCollider|SetLength _positionalcapsulecollider (Math|Conversions|ToFloat(Integer) (Variables|Default|GetLength)))
  (Variables|/Script/unreal_positional.PositionalCapsuleCollider|SetRadius _positionalcapsulecollider (Math|Conversions|ToFloat(Integer) (Variables|Default|GetRadius))))