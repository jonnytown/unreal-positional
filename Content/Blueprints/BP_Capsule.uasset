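; BP_Capsule is an actor that forms a capsule shape from three child actors: a Cylinder and two caps, sized by Radius and Length.
; BuildCapsule scales the parts on the assumption of 100-unit base shapes and moves the caps to either end of the cylinder, so Length excludes the caps.
; It runs from both the construction script and BeginPlay.
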(event EventBeginPlay
  (CallFunction|BuildCapsule))

(fn ConstructionScript
  (CallFunction|BuildCapsule))

(fn BuildCapsule
  (bind _length (Variables|Default|GetLength))
  (bind _radius (Variables|Default|GetRadius))
  (bind _cap1 (Variables|Default|Getcap1))
  (bind _cap2 (Variables|Default|Getcap2))
  (bind _returnvalue (/ _radius 5e+01))
  (bind _returnvalue_2 (/ _length 2.0))
  (bind _childactor (Variables|/Script/Engine.ChildActorComponent|GetChildActor _cap1))
  (bind _childactor_2 (Variables|/Script/Engine.ChildActorComponent|GetChildActor _cap2))
  (bind _returnvalue_3 (Math|Vector|MakeVector _returnvalue _returnvalue _returnvalue))
  (Transformation|SetActorRelativeScale3D (Variables|/Script/Engine.ChildActorComponent|GetChildActor (Variables|Default|Getcylinder)) (Math|Vector|MakeVector _returnvalue _returnvalue (/ _length 1e+02)))
  (Transformation|SetActorRelativeScale3D _childactor _returnvalue_3)
  (Transformation|SetActorRelativeLocation _childactor (Math|Vector|MakeVector 0.0 0.0 _returnvalue_2))
  (Transformation|SetActorRelativeScale3D _childactor_2 _returnvalue_3)
  (Transformation|SetActorRelativeLocation _childactor_2 (Math|Vector|MakeVector 0.0 0.0 (* _returnvalue_2 -1.0))))